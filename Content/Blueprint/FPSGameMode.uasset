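; FPS game mode Blueprint that runs a warmup countdown and tracks the remaining drones.
; BeginPlay creates the HUD, counts all DronePawn actors and caches the player's FPS_Character.
; During Warmup, Tick updates the countdown from game time, then hides it, enables player input and switches the session to InProgress.
; DroneDied decrements the count and refreshes the HUD; no end-of-game check follows.
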(event `self.ReceiveBeginPlay`
  (bind _returnvalue (`|CreateWidget` "/Game/Blueprint/GameModeHUD.GameModeHUD_C"))
  (bind _output_get (set `self.HUD` _returnvalue))
  (`UserWidget.AddToViewport` _output_get 0)
  (bind _outactors (`GameplayStatics.GetAllActorsOfClass` "/Game/Blueprint/DronePawn.DronePawn_C"))
  (bind _output_get_2 (set `self.DroneAmount` (`KismetArrayLibrary.Array_Length` _outactors)))
  (`TextBlock.SetText` (`/Game/Blueprint/GameModeHUD.DroneRemaining` (`self.HUD`)) (`KismetTextLibrary.Conv_IntToText` _output_get_2))
  (bind _asfps_character (cast `/Game/Blueprint/FPS_Character` (`GameplayStatics.GetPlayerPawn` 0)))
  (set `self.PlayerPawn` _asfps_character))

(event `self.ReceiveTick`
  (params (DeltaSeconds :type "Float (single-precision)"))
  (switch `/Game/Blueprint/ESessionStates` (`self.CurrentSessionState`)
    (:`NewEnumerator0`
      (`self.UpdateWarmupTimer`))))

(fn `DroneDied`
  (bind _output_get (set `self.DroneAmount` (- (`self.DroneAmount`) 1)))
  (`TextBlock.SetText` (`/Game/Blueprint/GameModeHUD.DroneRemaining` (`self.HUD`)) (`KismetTextLibrary.Conv_IntToText` _output_get)))

(fn `StartGame`
  (`Widget.SetVisibility` (`/Game/Blueprint/GameModeHUD.WarmupText` (`self.HUD`)) "Collapsed")
  (`/Game/Blueprint/FPS_Character.SwitchInputOn` (`self.PlayerPawn`) true)
  (set `self.CurrentSessionState` "NewEnumerator1"))

(fn `UpdateWarmupTimer`
  (bind _returnvalue (`KismetMathLibrary.FCeil64` (- (`self.WarmupTime`) (`KismetSystemLibrary.GetGameTimeInSeconds`))))
  (`TextBlock.SetText` (`/Game/Blueprint/GameModeHUD.WarmupText` (`self.HUD`)) (`KismetTextLibrary.Conv_Int64ToText` _returnvalue))
  (if (<= _returnvalue 0)
    (`self.StartGame`)))

(fn `UserConstructionScript`)